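; Weather controller Blueprint that advances the weather on a timer and shows the current weather as an image on a panel.
; InitWeatherController stores the WeatherPanel reference.
; Tick accumulates time and calls NextWeather, defined outside these graphs, once the total passes a threshold, with no reset shown here.
; ChangeImage switches on NowWeather as a string to set the panel's brush to the Weather or Rain texture.
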(event `self.ReceiveTick`
  (params (DeltaSeconds :type "Float (single-precision)"))
  (bind _output_get (set `self.totalTime` (+ DeltaSeconds (`self.totalTime`))))
  (if (> _output_get 3.0)
    (`self.NextWeather`)))

(event `self.ChangeImage`
  (switch `string` (`KismetStringLibrary.Conv_ByteToString` (`self.nowWeather`))
    (:`0`
      (set `/Game/HUD/Weather_Panel.showingImage` (`WidgetBlueprintLibrary.MakeBrushFromTexture` "/Game/HUD/Asset/weather.weather") (`self.WeatherPanel`)))
    (:`1`
      (set `/Game/HUD/Weather_Panel.showingImage` (`WidgetBlueprintLibrary.MakeBrushFromTexture` "/Game/HUD/Asset/rain.rain") (`self.WeatherPanel`)))))

(fn `InitWeatherController`
  (params (WeatherPanel :type "/Game/HUD/Weather_Panel Object Reference"))
  (set `self.WeatherPanel` WeatherPanel))

(fn `UserConstructionScript`)