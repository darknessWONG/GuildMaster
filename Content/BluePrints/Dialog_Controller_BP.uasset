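; Dialog controller Blueprint that feeds dialog lines to a HUD when its dialog button is clicked.
; Initialization stores the HUD and binds ChangeDialog to its button click event.
; Each click calls NextDialog, reads the Dialog data table row named after DialogIndex, appends its context to the HUD's Dialogs and shows them.
; A missing row yields the literal "finish" as the line.
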(event `HUDUpdated`
  (add `/Game/HUD/HUD_UI.DialogButtonCliecked` (`self.HUD`) (delegate `self.ChangeDialog`)))

(event `self.ChangeDialog`
  (`self.NextDialog`)
  (bind _context (`self.GetDialog`))
  (`KismetArrayLibrary.Array_Add` (`/Game/HUD/HUD_UI.Dialogs` (`self.HUD`)) _context)
  (`/Game/HUD/HUD_UI.ShowDialogs` (`self.HUD`)))

(fn `GetDialog`
  (returns (Context :type Text))
  (bind _returnvalue (`|GetDataTableRow` "/Game/Datatable/Dialog.Dialog" (`KismetStringLibrary.Conv_StringToName` (`KismetStringLibrary.Conv_IntToString` (`self.DialogIndex`))))
    (:`then`
      (return (`.Context_2_562F58534CCBADEF9609318A29D4C2D6` (break `/Game/Datatable/Dialog_Struct` _returnvalue))))
    (:`RowNotFound`
      (return "finish"))))

(fn `Initiailze_DialogControllerBP`
  (params (HUD :type "/Game/HUD/HUD_UI Object Reference"))
  (set `self.HUD` HUD)
  (`self.HUDUpdated`))

(fn `UserConstructionScript`)